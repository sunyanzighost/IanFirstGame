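; MainPlayerController_BP is a player controller Blueprint that animates the showing and hiding of the pause menu.
; Show calls the parent implementation, then casts the menu to PauseMenu and plays its PauseMenuAnimation forward.
; Hide plays that animation in reverse, then waits a fixed half-second delay before calling the parent implementation.
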(event `self.ShowPauseMenu`
  (`parent.ShowPauseMenu`)
  (bind _aspause_menu (cast `/Game/IanFirstGame/HUDs/PauseMenu` (`self.PauseMenu`)))
  (`UserWidget.PlayAnimation` _aspause_menu (`/Game/IanFirstGame/HUDs/PauseMenu.PauseMenuAnimation` _aspause_menu) 0.0 1 "Forward" 1.0 false))

(event `self.HidePauseMenu`
  (bind _aspause_menu (cast `/Game/IanFirstGame/HUDs/PauseMenu` (`self.PauseMenu`)))
  (`UserWidget.PlayAnimation` _aspause_menu (`/Game/IanFirstGame/HUDs/PauseMenu.PauseMenuAnimation` _aspause_menu) 0.0 1 "Reverse" 1.0 false)
  (`KismetSystemLibrary.Delay` 0.5)
  (`parent.HidePauseMenu`))

(fn `UserConstructionScript`)