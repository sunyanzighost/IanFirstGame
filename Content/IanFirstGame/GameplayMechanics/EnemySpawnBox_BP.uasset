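; Enemy spawn box that keeps an enemy in play by spawning one at a random point on BeginPlay and respawning it after death.
; Tick polls the spawned enemy's death state and, after a fixed Delay, spawns a replacement at a new random point.
; The SpawnEnemy override plays a burst particle effect at the location, then calls the parent implementation to do the actual spawn.
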(event `self.ReceiveBeginPlay`
  (`self.SpawnEnemy` (`self.Enemy`) (`self.GetRandomSpawnPoint`)))

(event `self.ReceiveTick`
  (params (DeltaSeconds :type "Float (single-precision)"))
  (bind _enemyspawned (`self.EnemySpawned`))
  (`/Engine/EditorBlueprintResources/StandardMacros.IsValid` _enemyspawned
    (:`Is Valid`
      (bind _returnvalue (`Enemy.IsDead` _enemyspawned))
      (if _returnvalue
        (`KismetSystemLibrary.Delay` 10.0)
        (`self.SpawnEnemy` (`self.Enemy`) (`self.GetRandomSpawnPoint`))))))

(event `self.SpawnEnemy`
  (params (EnemyClass :type "Object Class Reference") (SpawnLocation :type "Vector Structure (by ref)"))
  (`GameplayStatics.SpawnEmitterAtLocation` "/Game/InfinityBladeEffects/Effects/FX_Skill_RockBurst/P_RBurst_Default_Burst_Stalag_01.P_RBurst_Default_Burst_Stalag_01" SpawnLocation (struct) (1.0 1.0 1.0) false)
  (`parent.SpawnEnemy` EnemyClass SpawnLocation))

(fn `UserConstructionScript`)